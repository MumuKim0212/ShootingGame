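; BP_Player is the player actor in a shooter, moving along its right and up axes and firing bullets.
; Tick turns horizontal and vertical input into a normalized direction and sets the location without sweep.
; Holding Fire runs a looping timer on MakeBullet, which plays a sound and spawns BP_Bullet at the Arrow.
; DoDamage lowers HP through SetHP, which updates the WBP_PlayerHP widget, and returns whether HP is depleted.
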(event `self.ReceiveBeginPlay`
  (`self.SetHP` (`self.MaxHP`)))

(event `self.ReceiveTick`
  (params (DeltaSeconds :type "Float (single-precision)"))
  (`|ExecutionSequence`
    (:`then_0`
      (`self.Translate` (`self.GetDirection`) (`self.Speed`)))))

(event `InputAction|Fire`
  (params (Key :type "Key Structure"))
  ;[1 1 1] 마우스 왼쪽 버튼을 누르면 총알 액터를 하나 생성해서
  ; 총구위치에 배치하고 싶다.
)

(event `InputAction|Fire`
  (params (Key :type "Key Structure"))
  (:`Pressed`
    (bind _returnvalue (`KismetSystemLibrary.K2_SetTimer` null "MakeBullet" (`self.FireInterval`) true))
    (set `self.MakeBulletTimerHandle` _returnvalue)
    (`self.MakeBullet`))
  (:`Released`
    (`KismetSystemLibrary.K2_ClearAndInvalidateTimerHandle` (`self.MakeBulletTimerHandle`))))

(fn `DoDamage`
  (params (Damage :type Integer))
  (returns (isDie :type Boolean))
  (`self.SetHP` (- (`self.HP`) Damage))
  (return (<= (`self.HP`) 0)))

(fn `GetDirection`
  (returns (Direction :type "Vector Structure"))
  (return (`KismetMathLibrary.Normal` (+ (* (`self.GetInputAxisValue`) (`self.GetActorRightVector`)) (* (`self.GetInputAxisValue`) (`self.GetActorUpVector`))))))

(fn `MakeBullet`
  (`GameplayStatics.PlaySound2D` "/Game/VFX/FireSound.FireSound" 1.0 1.0 0.0 null null)
  (`|SpawnActorFromClass` "/Game/BluePrint/BP_Bullet.BP_Bullet_C" (`SceneComponent.K2_GetComponentToWorld` (`self.Arrow`)) "AlwaysSpawn" "MultiplyWithRoot" null null))

(fn `SetHP`
  (params (value :type Integer))
  (set `self.HP` value)
  (bind _aswbp_player_hp (cast `/Game/BluePrint/WBP_PlayerHP` (`WidgetComponent.GetWidget` (`self.WidgetHP`))))
  (`/Game/BluePrint/WBP_PlayerHP.UpdateHP` _aswbp_player_hp (`KismetMathLibrary.Conv_IntToDouble` (`self.HP`)) (`KismetMathLibrary.Conv_IntToDouble` (`self.MaxHP`))))

(fn `Translate`
  (params (Direction :type "Vector Structure") (Speed :type "Float (double-precision)"))
  (`self.K2_SetActorLocation` (+ (`self.K2_GetActorLocation`) (* Speed (`KismetMathLibrary.Normal` Direction) (`GameplayStatics.GetWorldDeltaSeconds`)))))

(fn `UserConstructionScript`)