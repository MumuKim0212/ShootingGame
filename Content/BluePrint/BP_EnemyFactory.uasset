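; BP_EnemyFactory is a spawner actor that repeatedly creates BP_Enemy instances at its Arrow component's world transform.
; BeginPlay starts a looping timer by function name at the MakeTime interval and stores its handle.
; MakeEnemy spawns regardless of collision while the player pawn is valid, otherwise it clears the timer to stop spawning.
; Tick-accumulator and random-delay event-timer alternatives remain in the graph but never run.
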(event `Event MakeEnemy`
  ;[1 1 1] 2. CustomEvent로 하는법
  (`self.Make Enemy`))

(event `self.ReceiveBeginPlay`
  (bind _returnvalue (`KismetSystemLibrary.K2_SetTimer` null "Make Enemy" (`self.MakeTime`) true))
  (set `self.TimerHandleMakeEnemy` _returnvalue))

(event `self.ReceiveTick`
  (params (DeltaSeconds :type "Float (single-precision)"))
  ;[1 1 1] 1. EventTick은 반복작업시 성능저하가 발생
)

(fn `Make Enemy`
  (`/Engine/EditorBlueprintResources/StandardMacros.IsValid` (`GameplayStatics.GetPlayerPawn` 0)
    (:`Is Valid`
      (`|SpawnActorFromClass` "/Game/BluePrint/BP_Enemy.BP_Enemy_C" (`SceneComponent.K2_GetComponentToWorld` (`self.Arrow`)) "AlwaysSpawn" "MultiplyWithRoot" null null))
    (:`Is Not Valid`
      (`KismetSystemLibrary.K2_ClearAndInvalidateTimerHandle` (`self.TimerHandleMakeEnemy`)))))

(fn `UserConstructionScript`)